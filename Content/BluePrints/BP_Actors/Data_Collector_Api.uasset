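; Actor that pulls product data from the BimQuote web API to price a Datasmith model and show element info.
; BeginPlay logs in via VaRest with hardcoded credentials, then fetches products behind a loading screen before showing the Main_Teleporter widget.
; It matches normalized material names from attached mesh actors to product names and totals their costs into the widget.
; Tick traces under the cursor to display the hovered element's material and category.
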(event `self.ReceiveBeginPlay`
  (bind _returnvalue (subsystem `VaRestSubsystem`))
  ;[1 1 1] Get Token
  (bind _returnvalue_2 (`VaRestSubsystem.DecodeJsonObject` _returnvalue "{ \n    \"identifier\":\"Omar\", \n    \"password\":\"Saleh199637\" \n}"))
  (`VaRestSubsystem.CallURL` _returnvalue "http://bimquote.herokuapp.com/api/auth/local" "POST" "x_www_form_urlencoded_body" _returnvalue_2 (delegate `CustomEvent_3`)))

(event `CustomEvent_3`
  (params (Request :type "VaRestRequestJSON Object Reference"))
  ;[1 1 1] Get Token
  (bind _output_get (set `self.TOKEN` (`VaRestJsonObject.GetStringField` (`VaRestRequestJSON.GetResponseObject` Request) "jwt")))
  ;[1 1 1] Comment
  (`|ExecutionSequence`
    (:`then_0`
      (bind _returnvalue (`VaRestSubsystem.ConstructVaRestRequestExt` (subsystem `VaRestSubsystem`) "GET" "x_www_form_urlencoded_url"))
      (`VaRestRequestJSON.SetHeader` _returnvalue "Authorization" (`KismetStringLibrary.Concat_StrStr` "Bearer " _output_get))
      (add `VaRestRequestJSON.OnRequestComplete` _returnvalue (delegate `CustomEvent_1`))
      (`VaRestRequestJSON.ProcessURL` _returnvalue "http://bimquote.herokuapp.com/api/front-end-objects-options?populate[Values][populate][Image][fields][0]=url"))
    (:`then_1`
      ;[1 1 1] Comment
      (bind _returnvalue_2 (`|CreateWidget` "/Game/BluePrints/Widgets/Loading_Screen/Loading_Screan.Loading_Screan_C"))
      (`UserWidget.AddToViewport` _returnvalue_2 0))))

(event `CustomEvent_1`
  (params (Request :type "VaRestRequestJSON Object Reference"))
  (bind _array_element_product_id (`self.Array Element Product Id`))
  ;[1 1 1] Comment
  (bind _output_get (set `self.All Objects_0` (`VaRestJsonObject.GetObjectArrayField` (`VaRestRequestJSON.GetResponseObject` Request) "data")))
  (for _array_element _output_get
    (`KismetArrayLibrary.Array_Add` (`self.attributes`) (make `/Game/BluePrints/Structs/attributes_struct_omar` (`VaRestJsonObject.GetObjectField` _array_element "attributes") (`VaRestJsonObject.GetIntegerField` _array_element "id"))))
  ;[1 1 1] Comment
  (for _array_element_2 (`self.attributes`)
    (for _array_element_3 (`VaRestJsonObject.GetObjectArrayField` (`VaRestJsonObject.GetObjectField` (break `/Game/BluePrints/Structs/attributes_struct_omar` _array_element_2) "Values") "data")
      (bind _returnvalue (`VaRestJsonObject.GetIntegerField` _array_element_3 "id"))
      (bind _returnvalue_2 (`KismetArrayLibrary.Array_AddUnique` _array_element_product_id _returnvalue))
      (if (`KismetArrayLibrary.Array_IsValidIndex` _array_element_product_id _returnvalue_2)
        (`KismetArrayLibrary.Array_Add` (`self.Product_Struct`) (make `/Game/BluePrints/Structs/Products_struct_omar` _array_element_3 _returnvalue (`VaRestJsonObject.GetStringField` (break `/Game/BluePrints/Structs/attributes_struct_omar` _array_element_2) "Category") (`VaRestJsonObject.GetStringField` (break `/Game/BluePrints/Structs/attributes_struct_omar` _array_element_2) "Subcategory") (`VaRestJsonObject.GetStringField` (break `/Game/BluePrints/Structs/attributes_struct_omar` _array_element_2) "Object_Name"))))))
  (`self.CustomEvent_2`)
  (`self.CustomEvent_0`))

(event `CustomEvent_2`
  ;[1 1 1] Comment
  (bind _foundwidgets (`WidgetBlueprintLibrary.GetAllWidgetsOfClass` "/Game/BluePrints/Widgets/Loading_Screen/Loading_Screan.Loading_Screan_C"))
  (`Widget.RemoveFromParent` (`|GetArrayItem` _foundwidgets))
  (bind _returnvalue (`|CreateWidget` "/Game/BluePrints/Widgets/Main_Teleporter/Main_Teleporter.Main_Teleporter_C"))
  (set `self.Teleporter` _returnvalue)
  (`UserWidget.AddToViewport` _returnvalue 0))

(event `self.ReceiveTick`
  (params (DeltaSeconds :type "Float (single-precision)"))
  (bind _teleporter (`self.Teleporter`))
  (bind _teleporter_2 (`self.Teleporter`))
  (bind _teleporter_3 (`self.Teleporter`))
  (bind _hitresult (`PlayerController.GetHitResultUnderCursorByChannel` (`GameplayStatics.GetPlayerController` 0) "TraceTypeQuery1" true))
  (bind _more_info (`/Game/BluePrints/Widgets/Main_Teleporter/Main_Teleporter.More_Info` _teleporter_3))
  (bind _more_info_2 (`/Game/BluePrints/Widgets/Main_Teleporter/Main_Teleporter.More_Info` _teleporter_2))
  ;[1 1 1] Comment
  (`/Engine/EditorBlueprintResources/StandardMacros.IsValid` _teleporter
    (:`Is Valid`
      (if (not (`/Game/BluePrints/Widgets/Main_Teleporter/Main_Teleporter.Is Clicked More Info2` _teleporter))
        (set `self.Hit Result Hit Actor` (`.HitActor` (`GameplayStatics.BreakHitResult` _hitresult)))
        (bind _returnvalue (`DatasmithContentBlueprintLibrary.GetDatasmithUserData` (`.HitActor` (`GameplayStatics.BreakHitResult` _hitresult))))
        (`/Engine/EditorBlueprintResources/StandardMacros.IsValid` _returnvalue
          (:`Is Valid`
            (`KismetSystemLibrary.PrintString` (`KismetSystemLibrary.GetDisplayName` (`.HitActor` (`GameplayStatics.BreakHitResult` _hitresult))) true true (struct :`G` 0.66 :`B` 1.0 :`A` 1.0) 0.0)
            (bind _asstatic_mesh_actor (cast `StaticMeshActor` (`.HitActor` (`GameplayStatics.BreakHitResult` _hitresult))))
            (bind _returnvalue_2 (`DatasmithContentBlueprintLibrary.GetDatasmithUserDataValueForKey` (`.HitActor` (`GameplayStatics.BreakHitResult` _hitresult)) "Element_Category"))
            (bind _output_get (set `self.Origenal Mat Name` (`KismetSystemLibrary.GetDisplayName` (`PrimitiveComponent.GetMaterial` (`StaticMeshActor.StaticMeshComponent` _asstatic_mesh_actor) 0))))
            (bind _returnvalue_3 (`self.get pure name` _output_get))
            (bind _output_get_2 (set `self.Mat_name` _returnvalue_3))
            (`KismetSystemLibrary.PrintString` _output_get_2 true true (struct :`G` 0.66 :`B` 1.0 :`A` 1.0) 0.0)
            (`/Engine/EditorBlueprintResources/StandardMacros.IsValid` (`self.Teleporter`)
              (:`Is Valid`
                (if (not (`KismetTextLibrary.TextIsEmpty` (`KismetTextLibrary.Conv_StringToText` (`self.Origenal Mat Name`))))
                  (`KismetSystemLibrary.Delay` 0.2)
                  (set `/Game/BluePrints/Widgets/Main_Teleporter/Main_Teleporter.In_Text` (`KismetTextLibrary.Conv_StringToText` (`self.Origenal Mat Name`)) _teleporter_2)
                  (set `/Game/BluePrints/Widgets/Main_Teleporter/Main_Teleporter.GetText_cat_name` (`KismetTextLibrary.Conv_StringToText` _returnvalue_2) _teleporter_2)
                  (if (not (`Widget.IsVisible` _more_info_2))
                    (`Widget.SetVisibility` _more_info_2 "SelfHitTestInvisible"))))))
          (:`Is Not Valid`
            (`/Engine/EditorBlueprintResources/StandardMacros.IsValid` _teleporter_3
              (:`Is Valid`
                (if (`Widget.IsVisible` _more_info)
                  (`KismetSystemLibrary.Delay` 0.2)
                  (`Widget.SetVisibility` _more_info "Hidden"))))))))))

(event `CustomEvent_0`
  (bind _names_from_model (`self.names from model`))
  ;[1 1 1] Comment
  (for _array_element (`self.Product_Struct`)
    (bind _returnvalue (`self.get pure name` (`VaRestJsonObject.GetStringField` (`VaRestJsonObject.GetObjectField` (break `/Game/BluePrints/Structs/Products_struct_omar` _array_element) "attributes") "Name")))
    (`KismetArrayLibrary.Array_Add` (`self.names from api`) _returnvalue))
  ;[1 1 1] Comment
  (for _array_element_2 (`self.GetAttachedActors` (`self.DataSmith Elements`) true)
    (bind _asstatic_mesh_actor (cast `StaticMeshActor` _array_element_2))
    (bind _returnvalue_2 (`self.get pure name` (`KismetSystemLibrary.GetDisplayName` (`PrimitiveComponent.GetMaterial` (`StaticMeshActor.StaticMeshComponent` _asstatic_mesh_actor) 0))))
    (`KismetArrayLibrary.Array_Add` (`self.names from model`) _returnvalue_2))
  ;[1 1 1] Comment
  (`/Game/SimpleFunctionsLibrary/SimpleFunctionsLibrary.Remove Non Unique Strings` _names_from_model)
  (for _array_element_3 _names_from_model
    (bind _returnvalue_3 (`KismetArrayLibrary.Array_Find` (`self.names from api`) _array_element_3))
    (if (not (== _returnvalue_3 -1))
      (bind _output_product (break `/Game/BluePrints/Structs/Products_struct_omar` (`|GetArrayItem` (`self.Product_Struct`) _returnvalue_3)))
      (set `self.Total Price` (+ (`VaRestJsonObject.GetNumberField` (`VaRestJsonObject.GetObjectField` _output_product "attributes") "Cost") (`self.Total Price`)))))
  (set `/Game/BluePrints/Widgets/Main_Teleporter/Main_Teleporter.Wid Total Price` (`KismetStringLibrary.Conv_DoubleToString` (`self.Total Price`)) (`self.Teleporter`)))

(fn `get pure name`
  (params (SourceString :type String))
  (returns (ReturnValue :type String))
  (return (`KismetSystemLibrary.MakeLiteralString` (`KismetStringLibrary.ToLower` (`KismetStringLibrary.Replace` (`KismetStringLibrary.Replace` (`KismetStringLibrary.Replace` (`KismetStringLibrary.Replace` SourceString "_" " ") " ") "-") "material")))))

(fn `UserConstructionScript`)