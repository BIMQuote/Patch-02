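; Level-control actor handling camera startup, cursor toggling, quitting and Pixel Streaming commands.
; BeginPlay blends to an actor picked by index, while a custom event, uncalled here, possesses the "Overview" CameraPawn and binds the streamer listener.
; Streamed JSON is routed by category to open levels by name or forward camera changes to the Main_Teleporter widget.
; Duplicated FlipFlop handlers create that widget and switch input mode, cursor and HUD.
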(event `InputAction|CtrlCourser`
  (params (Key :type "Key Structure"))
  (bind _returnvalue (`GameplayStatics.GetPlayerController` 0))
  (bind (_sizex _sizey) (`PlayerController.GetViewportSize` _returnvalue))
  (bind _returnvalue_2 (`PlayerController.GetHUD` _returnvalue))
  ;[1 1 1] Show / Hide Mouse
  (:`Pressed`
    (`/Engine/EditorBlueprintResources/StandardMacros.FlipFlop`
      (:`A`
        (bind _returnvalue_3 (`|CreateWidget` "/Game/BluePrints/Widgets/Main_Teleporter/Main_Teleporter.Main_Teleporter_C"))
        (`WidgetBlueprintLibrary.SetInputMode_GameAndUIEx` _returnvalue _returnvalue_3 "DoNotLock" false)
        (set `PlayerController.bShowMouseCursor` true _returnvalue)
        (set `HUD.bShowHUD` false _returnvalue_2)
        (`PlayerController.SetMouseLocation` _returnvalue (/ _sizex 2) (/ _sizey 2)))
      (:`B`
        (`WidgetBlueprintLibrary.SetInputMode_GameOnly` _returnvalue)
        (set `PlayerController.bShowMouseCursor` false _returnvalue)
        (set `HUD.bShowHUD` true _returnvalue_2)
        (`WidgetBlueprintLibrary.SetFocusToGameViewport`)))))

(event `self.ReceiveBeginPlay`
  (bind _returnvalue (`GameplayStatics.GetPlayerController` 0))
  ;[1 1 1] Comment
  (`|ExecutionSequence`
    (:`then_0`
      (bind _outactors (`GameplayStatics.GetAllActorsOfClass` null))
      (`PlayerController.SetViewTargetWithBlend` _returnvalue (`|GetArrayItem` _outactors 3) 1.0 "VTBlend_Linear" 0.0 false)
      (`KismetSystemLibrary.Delay` 1.5)
      (`Controller.Possess` _returnvalue null))))

(event `InputAction|Quie`
  (params (Key :type "Key Structure"))
  ;[1 1 1] quite form game
  (:`Pressed`
    (`KismetSystemLibrary.QuitGame` null "Quit")))

(event `InputAction|CtrlCourser`
  (params (Key :type "Key Structure"))
  (bind _returnvalue (`GameplayStatics.GetPlayerController` 0))
  (bind _returnvalue_2 (`PlayerController.GetHUD` _returnvalue))
  (bind (_sizex _sizey) (`PlayerController.GetViewportSize` _returnvalue))
  ;[1 1 1] Show / Hide Mouse
  (:`Pressed`
    (`/Engine/EditorBlueprintResources/StandardMacros.FlipFlop`
      (:`A`
        (bind _returnvalue_3 (`|CreateWidget` "/Game/BluePrints/Widgets/Main_Teleporter/Main_Teleporter.Main_Teleporter_C"))
        (`WidgetBlueprintLibrary.SetInputMode_GameAndUIEx` _returnvalue _returnvalue_3 "DoNotLock" false)
        (set `PlayerController.bShowMouseCursor` true _returnvalue)
        (set `HUD.bShowHUD` false _returnvalue_2))
      (:`B`
        (`WidgetBlueprintLibrary.SetInputMode_GameOnly` _returnvalue)
        (set `PlayerController.bShowMouseCursor` false _returnvalue)
        (set `HUD.bShowHUD` true _returnvalue_2)
        (`WidgetBlueprintLibrary.SetFocusToGameViewport`)))
    (`PlayerController.SetMouseLocation` _returnvalue (/ _sizex 2) (/ _sizey 2))))

(event `CustomEvent`
  (bind _returnvalue (`GameplayStatics.GetPlayerController` 0))
  ;[1 1 1] Comment
  (`|ExecutionSequence`
    (:`then_0`
      (bind _outactors (`GameplayStatics.GetAllActorsOfClass` "/Game/BluePrints/GameMode/CameraPawn.CameraPawn_C"))
      (for _array_element _outactors
        (if (`KismetStringLibrary.EqualEqual_StrStr` (`KismetSystemLibrary.GetDisplayName` _array_element) "Overview")
          (`PlayerController.SetViewTargetWithBlend` _returnvalue _array_element 1.0 "VTBlend_Linear" 0.0 false)
          (`KismetSystemLibrary.Delay` 1.5)
          (`Controller.Possess` _returnvalue _array_element)
          (break))))
    (:`then_1`
      ;[1 1 1] Comment
      (add `PixelStreamerInputComponent.OnInputEvent` (`self.PixelStreamerInput`) (delegate `CustomEvent_0`))
      (`WidgetBlueprintLibrary.SetFocusToGameViewport`))))

(event `CustomEvent_0`
  (params (Descriptor :type String))
  (bind _stringvalue (`PixelStreamerInputComponent.GetJsonStringValue` (`self.PixelStreamerInput`) (`self.Descriptor`) "Sub_category"))
  (bind _stringvalue_2 (`PixelStreamerInputComponent.GetJsonStringValue` (`self.PixelStreamerInput`) (`self.Descriptor`) "Level_number"))
  ;[1 1 1] Comment
  (bind _output_get (set `self.Descriptor` Descriptor))
  (bind (_stringvalue_3 _success) (`PixelStreamerInputComponent.GetJsonStringValue` (`self.PixelStreamerInput`) _output_get "Category"))
  (if _success
    (`KismetSystemLibrary.PrintString` _stringvalue_3 true true (struct :`R` 1.0 :`G` 0.033889 :`A` 1.0) 500.0)
    (switch `string` _stringvalue_3
      (:`0`
        (`KismetSystemLibrary.PrintString` _stringvalue true true (struct :`G` 0.66 :`B` 1.0 :`A` 1.0) 500.0)
        (switch `string` _stringvalue
          (:`Level_selector`
            (`KismetSystemLibrary.PrintString` _stringvalue_2 true true (struct :`R` 0.43897 :`G` 0.281627 :`B` 1.0 :`A` 1.0) 500.0)
            (`GameplayStatics.OpenLevel` (`KismetStringLibrary.Conv_StringToName` _stringvalue_2)))))
      (:`1`
        (`KismetSystemLibrary.PrintString` _stringvalue true true (struct :`R` 0.391056 :`G` 1.0 :`A` 1.0) 500.0)
        (switch `string` _stringvalue
          (:`Cameras`
            (bind _foundwidgets (`WidgetBlueprintLibrary.GetAllWidgetsOfClass` "/Game/BluePrints/Widgets/Main_Teleporter/Main_Teleporter.Main_Teleporter_C"))
            (bind _output_get_2 (set `self.Camera-name` (`PixelStreamerInputComponent.GetJsonStringValue` (`self.PixelStreamerInput`) (`self.Descriptor`) "Camera_name")))
            (`KismetSystemLibrary.PrintString` _output_get_2 true true (struct :`R` 0.43897 :`G` 0.281627 :`B` 1.0 :`A` 1.0) 500.0)
            (message `/Game/BluePrints/GameMode/NewInterface_Omar.Change Camea` (`|GetArrayItem` _foundwidgets))))))))

(fn `UserConstructionScript`)