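; Player controller for a Pixel Streaming building viewer, driven by JSON commands to open levels, switch cameras and swap materials or meshes.
; BeginPlay sets up the cursor, possesses the Overview camera, caches CameraPawns and asset-registry lists, and binds the input event.
; Camera switches blend and fade, then possess on a timer.
; Swaps convert the keyword's underscores to hyphens, match game-mode data table rows, and find actors by Revit element ID tags.
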(event `self.ReceiveBeginPlay`
  (bind _returnvalue (`GameplayStatics.GetPlayerController` 0))
  (bind _returnvalue_2 (`GameplayStatics.GetPlayerController` 0))
  (bind _returnvalue_3 (`GameplayStatics.GetPlayerController` 0))
  (bind (_sizex _sizey) (`self.GetViewportSize` _returnvalue))
  (`|ExecutionSequence`
    (:`then_0`
      ;[1 1 1] Show / Hide Mouse
      (bind _returnvalue_4 (`|CreateWidget` "/Game/BluePrints/Widgets/Mouse/Mouse_Cursor.Mouse_Cursor_C" _returnvalue_2))
      (`self.SetMouseCursorWidget` _returnvalue_2 "None" _returnvalue_4)
      (`WidgetBlueprintLibrary.SetInputMode_GameAndUIEx` _returnvalue null "DoNotLock" false)
      (`self.SetMouseLocation` _returnvalue (/ _sizex 2) (/ _sizey 2)))
    (:`then_1`
      ;[1 1 1] Comment
      (bind _outactors (`GameplayStatics.GetAllActorsOfClass` "/Game/BluePrints/GameMode/CameraPawn.CameraPawn_C"))
      (bind _output_get (set `self.Out Actors - All Cameras Actors` _outactors))
      (for _array_element _output_get
        (if (`KismetStringLibrary.EqualEqual_StrStr` (`/Game/BluePrints/GameMode/CameraPawn.Camera_name` _array_element) "Overview")
          (`self.SetViewTargetWithBlend` _returnvalue_3 _array_element 1.0 "VTBlend_Linear" 0.0 false)
          (`|ExecutionSequence`
            (:`then_0`
              (`KismetSystemLibrary.Delay` 1.5)
              (`self.Possess` _returnvalue_3 _array_element)
              (break))
            (:`then_1`
              (break))))))
    (:`then_2`
      ;[1 1 1] Comment
      (for (_array_element_2 _array_index) (`self.Out Actors - All Cameras Actors`)
        (`KismetArrayLibrary.Array_Add` (`self.All Camera Pawn Struct`) (make `/Game/BluePrints/Structs/All_Camera_pawn_Struct_Omar` _array_index (`/Game/BluePrints/GameMode/CameraPawn.Camera_name` _array_element_2) _array_element_2))))
    (:`then_3`
      ;[0 0 0] Get Materials
      (bind _asgame_mode_omar (cast `/Game/BluePrints/GameMode/GameMode_Omar` (`GameplayStatics.GetGameMode`)))
      (bind _globaldirectories_materialspath (break `/Game/BluePrints/Structs/GlobalDirectoriesStruct` (`/Game/BluePrints/GameMode/GameMode_Omar.GlobalDirectories` _asgame_mode_omar)))
      (bind (_outassetdata _returnvalue_5) (`AssetRegistry.GetAssetsByPath` (`AssetRegistryHelpers.GetAssetRegistry`) _globaldirectories_materialspath true false))
      (if _returnvalue_5
        (set `self.MaterialsArray` _outassetdata)))
    (:`then_4`
      ;[1 1 1] Comment
      (add `PixelStreamerInputComponent.OnInputEvent` (`self.PixelStreamerInput`) (delegate `PixelStreamerInputEvent`))
      (`WidgetBlueprintLibrary.SetFocusToGameViewport`))
    (:`then_5`
      ;[0 0 0] Get Level Static Meshes
      (bind _outactors_2 (`GameplayStatics.GetAllActorsOfClass` "/Game/BluePrints/GameMode/GameMode_Omar.GameMode_Omar_C"))
      (bind _levelstaticmeshes_path (`/Game/BluePrints/GameMode/GameMode_Omar.GetLevelStaticMeshesPath` (`|GetArrayItem` _outactors_2)))
      (bind (_outassetdata_2 _returnvalue_6) (`AssetRegistry.GetAssetsByPath` (`AssetRegistryHelpers.GetAssetRegistry`) _levelstaticmeshes_path true false))
      (if _returnvalue_6
        (set `self.LevelStaticMeshesArray` _outassetdata_2)))))

(event `PixelStreamerInputEvent`
  (params (Descriptor :type String))
  (bind _stringvalue (`PixelStreamerInputComponent.GetJsonStringValue` (`self.PixelStreamerInput`) (`self.Descriptor`) "Sub_category"))
  (bind _stringvalue_2 (`PixelStreamerInputComponent.GetJsonStringValue` (`self.PixelStreamerInput`) (`self.Descriptor`) "Sub_category"))
  (bind _stringvalue_3 (`PixelStreamerInputComponent.GetJsonStringValue` (`self.PixelStreamerInput`) (`self.Descriptor`) "Level_number"))
  ;[1 1 1] Comment
  (bind _output_get (set `self.Descriptor` Descriptor))
  (bind (_stringvalue_4 _success) (`PixelStreamerInputComponent.GetJsonStringValue` (`self.PixelStreamerInput`) _output_get "Category"))
  (if _success
    (`KismetSystemLibrary.PrintString` (`KismetStringLibrary.Concat_StrStr` "Category = " _stringvalue_4) true true (struct :`R` 1.0 :`G` 0.033889 :`A` 1.0))
    (`self.SetPixelStreamingDescriptorAssociatedVariables`)
    (switch `string` _stringvalue_4
      (:`0`
        ;[1 1 1] Open Levels
        (`KismetSystemLibrary.PrintString` _stringvalue)
        (switch `string` _stringvalue
          (:`Level_selector`
            (`KismetSystemLibrary.PrintString` _stringvalue_3 true true (struct :`R` 0.43897 :`G` 0.281627 :`B` 1.0 :`A` 1.0) 500.0)
            (`GameplayStatics.OpenLevel` (`KismetStringLibrary.Conv_StringToName` _stringvalue_3)))))
      (:`1`
        ;[1 1 1] Camera
        (`KismetSystemLibrary.PrintString` _stringvalue_2 true true (struct :`R` 0.391056 :`G` 1.0 :`A` 1.0))
        (switch `string` _stringvalue_2
          (:`Cameras`
            (bind _output_get_2 (set `self.Camera-name-From-Varest` (`PixelStreamerInputComponent.GetJsonStringValue` (`self.PixelStreamerInput`) (`self.Descriptor`) "Camera_name")))
            (`KismetSystemLibrary.PrintString` _output_get_2 true true (struct :`R` 0.43897 :`G` 0.281627 :`B` 1.0 :`A` 1.0) 500.0)
            (`self.Teleport Camera`))))
      (:`2`
        ;[0 0 0] Change Materials
        (`|ExecutionSequence`
          (:`then_0`
            (`self.ApplyKeywordDatabaseFormat`))
          (:`then_1`
            (`self.MaterialDebugLog`))
          (:`then_2`
            (for _array_element (`self.MaterialsArray`)
              (bind _returnvalue (`AssetRegistryHelpers.GetAsset` _array_element))
              (if (`KismetStringLibrary.EqualEqual_StrStr` (`KismetSystemLibrary.GetObjectName` _returnvalue) (`self.Material Name`))
                (bind _asmaterial_instance (cast `MaterialInstance` _returnvalue))
                (set `self.Material Instance` _asmaterial_instance)
                (break)))
            (bind _actorswithkeyastag (`self.GetAllActorsWithKey` (`self.Keyword`)))
            ;;[0 0 0] Change Actor Static Mesh Materials
            (for _array_element_2 _actorswithkeyastag
              (bind _asstatic_mesh_actor (cast `StaticMeshActor` _array_element_2))
              (bind _staticmeshcomponent (`StaticMeshActor.StaticMeshComponent` _asstatic_mesh_actor))
              (bind _index (`/SortPlugin/Blueprints/ArrayHelperMacrosLibrary.ForLoopStep` 0 (- (`PrimitiveComponent.GetNumMaterials` _staticmeshcomponent) 1))
                (:`LoopBody`
                  (`PrimitiveComponent.SetMaterial` _staticmeshcomponent _index (`self.Material Instance`))))))))
      (:`3`
        ;[0 0 0] Change Types
        (`|ExecutionSequence`
          (:`then_0`
            (`self.ApplyKeywordDatabaseFormat`))
          (:`then_1`
            (`self.DescriptorAssociatedVariablesDebugLog`))
          (:`then_2`
            (for _array_element_3 (`self.LevelStaticMeshesArray`)
              (bind _returnvalue_2 (`AssetRegistryHelpers.GetAsset` _array_element_3))
              (if (`KismetStringLibrary.EqualEqual_StrStr` (`KismetSystemLibrary.GetObjectName` _returnvalue_2) (`self.Material Name`))
                (bind _asstatic_mesh (cast `StaticMesh` _returnvalue_2))
                (set `self.As Static Mesh` _asstatic_mesh)
                (break)))
            (bind _actorswithkeyastag_2 (`self.GetAllActorsWithKey` (`self.Keyword`) "NewEnumerator1"))
            ;;[0 0 0] Change Static Mesh
            (for _array_element_4 _actorswithkeyastag_2
              (bind _asstatic_mesh_actor_2 (cast `StaticMeshActor` _array_element_4))
              (`StaticMeshActor.SetMobility` _asstatic_mesh_actor_2 "Stationary")
              (`StaticMeshComponent.SetStaticMesh` (`StaticMeshActor.StaticMeshComponent` _asstatic_mesh_actor_2) (`self.As Static Mesh`)))))))))

(event `Key|X`
  (params (Key :type "Key Structure"))
  (:`Pressed`
    (bind (_new_descriptor _success) (`self.SendDataToUnreal_ACloneFunction` "2" "Roof?Roof_Material?AnyRequiredData?LivingFurnitureChair" "UC_Aluminum_Shingle" "28_1200" "SW_Dewberry"))
    ;[1 1 1] Comment
    (if _success
      _)))

(event `Key|Q`
  (params (Key :type "Key Structure"))
  ;[0 0 0] Debugging (Safe to be deleted)
)

(event `Teleport Camera`
  (bind _returnvalue (`GameplayStatics.GetPlayerController` 0))
  ;[1 1 1] Camera Teleporter
  (if (not (`KismetSystemLibrary.K2_IsTimerActiveHandle` (`self.Timer`)))
    (for _array_element (`self.All Camera Pawn Struct`)
      (if (`KismetStringLibrary.EqualEqual_StrStr` (`.Name_8_B5FA8B324851DED95DA0EA81DAF07744` (break `/Game/BluePrints/Structs/All_Camera_pawn_Struct_Omar` _array_element)) (`self.Camera-name-From-Varest`))
        (`|ExecutionSequence`
          (:`then_0`
            (`self.SetViewTargetWithBlend` _returnvalue (`.CameraPawn_2_585E51BA48B4010D00B7F78643A7FB13` (break `/Game/BluePrints/Structs/All_Camera_pawn_Struct_Omar` _array_element)) 1.0 "VTBlend_Linear" 0.0 false)
            (`PlayerCameraManager.StartCameraFade` :`self` (`PlayerController.PlayerCameraManager` _returnvalue) :`ToAlpha` 1.0 :`Duration` 1.1)
            (bind _returnvalue_2 (`KismetSystemLibrary.K2_SetTimerDelegate` (delegate `Posess Timer`) 1.0))
            (set `self.Timer` _returnvalue_2))
          (:`then_1`
            (break)))))))

(event `Posess Timer`
  ;[1 1 1] Camera Teleporter
  (`self.Possess` (`GameplayStatics.GetPlayerController` 0) (`.CameraPawn_2_585E51BA48B4010D00B7F78643A7FB13` (break `/Game/BluePrints/Structs/All_Camera_pawn_Struct_Omar` (stale `Teleport Camera` _array_element)))))

(fn `ApplyKeywordDatabaseFormat`
  (set `self.Keyword` (`KismetStringLibrary.Replace` (`self.Keyword`) "_" "-")))

(fn `DescriptorAssociatedVariablesDebugLog`
  (`KismetSystemLibrary.PrintString` (`KismetStringLibrary.Concat_StrStr` "Sub_category = " (`self.Discriptor Sub Category`)))
  (`KismetSystemLibrary.PrintString` (`KismetStringLibrary.Concat_StrStr` "SC_Category = " (`self.Category`)))
  (`KismetSystemLibrary.PrintString` (`KismetStringLibrary.Concat_StrStr` "SC_SubCategory = " (`self.Sub Category`)))
  (`KismetSystemLibrary.PrintString` (`KismetStringLibrary.Concat_StrStr` "SC_AnyRequiredData = " (`self.AnyRequiredData`)))
  (`KismetSystemLibrary.PrintString` (`KismetStringLibrary.Concat_StrStr` "SC_Keyword = " (`self.Keyword`)))
  (`KismetSystemLibrary.PrintString` (`KismetStringLibrary.Concat_StrStr` "Material Name / StaticMesh Name = " (`self.Material Name`))))

(fn `Get Actors Using Key From Datatable`
  (params (DataTable :type "DataTable Object Reference") (Key :type String))
  (returns (ActorsWithKeyTag :type "Array of Actor Object Reference"))
  (locals (Actors :type "Array of Actor Object Reference"))
  (bind _outrownames (`DataTableFunctionLibrary.GetDataTableRowNames` DataTable)) ; Get all row names
  (for _array_element _outrownames
    (bind _returnvalue (`|GetDataTableRow` DataTable _array_element)
      (:`then`
        (if (`KismetStringLibrary.EqualEqual_StrStr` (`.Key_2_C0262A2F4ABD7CC8F28098A040ABBE99` (break `/Game/BluePrints/Structs/PixelStreamingKeys` _returnvalue)) Key)
          (bind _outactors (`GameplayStatics.GetAllActorsWithTag` (`KismetStringLibrary.Conv_StringToName` (`KismetStringLibrary.Concat_StrStr` "Revit.Element.Id." (`KismetStringLibrary.Conv_NameToString` _array_element))))) ; Get all actors that have this Key as tag
          (for _array_element_2 _outactors
            (`KismetArrayLibrary.Array_AddUnique` (`local.Actors`) _array_element_2))))))
  (return (`local.Actors`)))

(fn `Get Actors Using Key From Datatables`
  (params (DataTables :type "Array of DataTable Object Reference") (Key :type String))
  (returns (ActorsWithKeyTag :type "Array of Actor Object Reference"))
  (locals (Actors :type "Array of Actor Object Reference"))
  (for _array_element DataTables
    (bind _outrownames (`DataTableFunctionLibrary.GetDataTableRowNames` _array_element)) ; Get all row names
    (for _array_element_2 _outrownames
      (bind _returnvalue (`|GetDataTableRow` _array_element _array_element_2)
        (:`then`
          (if (`KismetStringLibrary.EqualEqual_StrStr` (`.Key_2_C0262A2F4ABD7CC8F28098A040ABBE99` (break `/Game/BluePrints/Structs/PixelStreamingKeys` _returnvalue)) Key)
            (bind _outactors (`GameplayStatics.GetAllActorsWithTag` (`KismetStringLibrary.Conv_StringToName` (`KismetStringLibrary.Concat_StrStr` "Revit.Element.Id." (`KismetStringLibrary.Conv_NameToString` _array_element_2))))) ; Get all actors that have this Key as tag
            (for _array_element_3 _outactors
              (`KismetArrayLibrary.Array_AddUnique` (`local.Actors`) _array_element_3)))))))
  (return (`local.Actors`)))

(fn `GetAllActorsWithKey`
  (params (Key :type String) (ChangeType :type "/Game/BluePrints/Enums/EChangeType Enum" :default "NewEnumerator0"))
  (returns (ActorsWithKeyAsTag :type "Array of Actor Object Reference"))
  (locals (CM_Actors :type "Array of Actor Object Reference"))
  (bind _returnvalue (`GameplayStatics.GetGameMode`))
  (switch `/Game/BluePrints/Enums/EChangeType` ChangeType
    (:`NewEnumerator0`
      (bind _levelpixelstreamingchangematerialkeysdatatable (message `/Game/BluePrints/Interfaces/BPI_PixelStreamingKeys.Get_LevelCorresponding_PixelStreaming_ChangeMaterialKeysDataTables` _returnvalue))
      (bind _actorswithkeytag (`self.Get Actors Using Key From Datatables` _levelpixelstreamingchangematerialkeysdatatable Key))
      (return _actorswithkeytag))
    (:`NewEnumerator1`
      (bind _levelpixelstreamingchangetypekeysdatatable (message `/Game/BluePrints/Interfaces/BPI_PixelStreamingKeys.Get_LevelCorresponding_PixelStreaming_ChangeTypeKeysDataTable` _returnvalue))
      (bind _actorswithkeytag_2 (`self.Get Actors Using Key From Datatable` _levelpixelstreamingchangetypekeysdatatable Key))
      (return _actorswithkeytag_2))))

(fn `MaterialDebugLog`
  (`self.DescriptorAssociatedVariablesDebugLog`)
  ;[0 0 0] Debug Get Actors With Key As Tag
  (bind _actorswithkeyastag (`self.GetAllActorsWithKey` (`self.Keyword`)))
  (`KismetSystemLibrary.PrintString` (`KismetStringLibrary.Concat_StrStr` "ActorsWithKey (Length) = " (`KismetStringLibrary.Conv_IntToString` (`KismetArrayLibrary.Array_Length` _actorswithkeyastag))))
  (for _array_element _actorswithkeyastag
    (`KismetSystemLibrary.PrintString` (`KismetSystemLibrary.GetDisplayName` _array_element) false)))

(fn `SendDataToUnreal_ACloneFunction`
  (params (Category :type String) (Sub_category :type String) (Camera_name :type String) (Level_number :type String) (`Mat_Name/StaticMeshName` :type String))
  (returns (`New Descriptor` :type String) (Success :type Boolean))
  (locals (LocalDiscriptor :type String))
  (bind _pixelstreamerinput (`self.PixelStreamerInput`))
  (bind (_newdescriptor _success) (`PixelStreamerInputComponent.AddJsonStringValue` _pixelstreamerinput (`local.LocalDiscriptor`) "Category" Category))
  (bind (_newdescriptor_2 _success_2) (`PixelStreamerInputComponent.AddJsonStringValue` _pixelstreamerinput _newdescriptor "Sub_category" Sub_category))
  (bind (_newdescriptor_3 _success_3) (`PixelStreamerInputComponent.AddJsonStringValue` _pixelstreamerinput _newdescriptor_2 "Camera_name" Camera_name))
  (bind (_newdescriptor_4 _success_4) (`PixelStreamerInputComponent.AddJsonStringValue` _pixelstreamerinput _newdescriptor_3 "Level_number" Level_number))
  (bind (_newdescriptor_5 _success_5) (`PixelStreamerInputComponent.AddJsonStringValue` _pixelstreamerinput _newdescriptor_4 "Mat_Name" `Mat_Name/StaticMeshName`))
  (return _newdescriptor_5 (and _success _success_2 _success_3 _success_4 _success_5)))

(fn `SetPixelStreamingDescriptorAssociatedVariables`
  (bind _descriptor (`self.Descriptor`))
  (bind _pixelstreamerinput (`self.PixelStreamerInput`))
  (bind _stringvalue (`PixelStreamerInputComponent.GetJsonStringValue` _pixelstreamerinput _descriptor "Sub_category"))
  (bind (_category _subcategory _anyrequireddata _keyword) (`self.Get Data From SubCategory Descriptor` _stringvalue "?"))
  (set `self.Discriptor Sub Category` _stringvalue)
  (set `self.Material Name` (`PixelStreamerInputComponent.GetJsonStringValue` _pixelstreamerinput _descriptor "Mat_Name"))
  (set `self.Category` _category)
  (set `self.Sub Category` _subcategory)
  (set `self.AnyRequiredData` _anyrequireddata)
  (set `self.Keyword` _keyword))

(fn `UserConstructionScript`)