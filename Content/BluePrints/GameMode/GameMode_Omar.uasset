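; GameMode that resolves per-level content paths and the PixelStreaming key DataTables for changing materials and types.
; It derives the level name from the map name after an underscore and builds that level's Geometries folder path, which BeginPlay prints.
; An Asset Registry scan recursively gathers DataTables from global directories.
; Material tables match when their names contain the level name; the type table lookup seeks a case-insensitive exact match.
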(event `self.ReceiveBeginPlay`
  (bind _levelstaticmeshes_path (`self.GetLevelStaticMeshesPath`))
  (`KismetSystemLibrary.PrintString` (`KismetStringLibrary.Conv_NameToString` _levelstaticmeshes_path)))

(fn `Get_LevelCorresponding_PixelStreaming_ChangeMaterialKeysDataTables`
  (returns (LevelPixelStreamingChangeMaterialKeysDataTable :type "Array of DataTable Object Reference"))
  (locals (DataTables :type "Array of DataTable Object Reference"))
  (bind (_globaldirectories_materialspath _globaldirectories_exteriorfloorsdatatablespath _globaldirectories_changematerialskeysdatatablespath) (break `/Game/BluePrints/Structs/GlobalDirectoriesStruct` (`self.GlobalDirectories`)))
  (bind _levelname (`self.GetLevelName`))
  (bind _pixelstreamingkeysdatatables (`self.Get_PixelStreamingKeys_DataTablesFromDirectory` _globaldirectories_changematerialskeysdatatablespath))
  (for _array_element _pixelstreamingkeysdatatables
    (if (`KismetStringLibrary.Contains` (`KismetSystemLibrary.GetDisplayName` _array_element) _levelname)
      (`KismetArrayLibrary.Array_AddUnique` (`local.DataTables`) _array_element)))
  (return (`local.DataTables`)))

(fn `Get_LevelCorresponding_PixelStreaming_ChangeTypeKeysDataTable`
  (returns (LevelPixelStreamingChangeTypeKeysDataTable :type "DataTable Object Reference"))
  (bind (_globaldirectories_materialspath _globaldirectories_exteriorfloorsdatatablespath _globaldirectories_changematerialskeysdatatablespath _globaldirectories_changetypeskeysdatatablespath) (break `/Game/BluePrints/Structs/GlobalDirectoriesStruct` (`self.GlobalDirectories`)))
  (bind _levelname (`self.GetLevelName`))
  (bind _pixelstreamingkeysdatatables (`self.Get_PixelStreamingKeys_DataTablesFromDirectory` _globaldirectories_changetypeskeysdatatablespath))
  (for _array_element _pixelstreamingkeysdatatables
    (if (`KismetStringLibrary.EqualEqual_StrStr` (`KismetStringLibrary.ToLower` (`KismetSystemLibrary.GetDisplayName` _array_element)) (`KismetStringLibrary.ToLower` _levelname))
      (break)))
  (return _array_element))

(fn `Get_PixelStreamingKeys_DataTablesFromDirectory`
  (params (Directory :type Name))
  (returns (PixelStreamingKeysDataTables :type "Array of DataTable Object Reference"))
  (bind _out_datatables (`self.GetDataTablesFromPath` Directory))
  (return _out_datatables))

(fn `GetDataTablesFromPath`
  (params (Directory :type Name))
  (returns (`Out DataTables` :type "Array of DataTable Object Reference"))
  (locals (DataTablesArray :type "Array of DataTable Object Reference"))
  (bind (_outassetdata _returnvalue) (message `AssetRegistry.GetAssetsByPath` (`KismetSystemLibrary.Conv_InterfaceToObject` (`AssetRegistryHelpers.GetAssetRegistry`)) Directory true false))
  (if _returnvalue
    (for _array_element _outassetdata
      (if (== (`AssetRegistryHelpers.GetClass` _array_element) "/Script/Engine.DataTable")
        (bind _asdata_table (cast `DataTable` (`AssetRegistryHelpers.GetAsset` _array_element)))
        (`KismetArrayLibrary.Array_AddUnique` (`local.DataTablesArray`) _asdata_table)))
    (return (`local.DataTablesArray`))))

(fn `GetLevelName`
  (returns (LevelName :type String))
  (bind _returnvalue (`GameplayStatics.GetCurrentLevelName` true))
  (bind (_lefts _rights _returnvalue_2) (`KismetStringLibrary.Split` _returnvalue "_"))
  (if _returnvalue_2
    (return _rights)))

(fn `GetLevelStaticMeshesPath`
  (returns (`LevelStaticMeshes Path` :type Name))
  (bind _returnvalue (`GameplayStatics.GetCurrentLevelName` true)) ; MapName
  (bind _levelname (`self.GetLevelName`)) ; LevelName
  (return (`KismetStringLibrary.Conv_StringToName` (`KismetStringLibrary.Concat_StrStr` "/Game/Maps/" _returnvalue "/" _levelname "_Craftsman_Exterior-3DView-_3D_/Geometries"))))

(fn `UserConstructionScript`)